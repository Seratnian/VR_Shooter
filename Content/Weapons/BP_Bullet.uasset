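; Bullet Blueprint that applies custom damping to its physics Body along the original direction of travel.
; Tick stores the Body's velocity in OriginalVelocity while that value is still near zero.
; Each tick it adds a force along that unnormalized vector, scaled by negative ForwardDamping, delta time and its dot product with current velocity.
; It also prints these values every tick.
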(event `self.ReceiveTick`
  (params (DeltaSeconds :type "Float (single-precision)"))
  (bind _body (`self.Body`))
  (bind _original_velocity (`self.Original Velocity`))
  (bind _returnvalue (`SceneComponent.GetComponentVelocity` _body))
  (bind _returnvalue_2 (* DeltaSeconds -1.0 (`self.Forward Damping`) (`KismetMathLibrary.Dot_VectorVector` _returnvalue _original_velocity)))
  (if (== (`self.Original Velocity`) (0.0 0.0 0.0))
    (set `self.Original Velocity` _returnvalue))
  (`KismetSystemLibrary.PrintString` (`KismetStringLibrary.Concat_StrStr` "Velocity " (`KismetStringLibrary.Conv_VectorToString` _original_velocity) " delta sec " (`KismetStringLibrary.Conv_DoubleToString` DeltaSeconds) " result " (`KismetStringLibrary.Conv_DoubleToString` _returnvalue_2)))
  (`PrimitiveComponent.AddForce` _body (* _original_velocity _returnvalue_2) "None" false))

(fn `UserConstructionScript`)