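; BP_Assault is an assault weapon Blueprint that fires automatically while the trigger is held.
; Pulling the trigger sets IsFiring, calls Fire immediately regardless of any remaining cooldown, and resets StillToWait to ShootTime.
; Tick runs the parent tick, counts StillToWait down and jumps back into that fire step when it expires, until release clears IsFiring.
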(event `self.TriggerPulled`
  (params (Controller :type "/Game/VirtualRealityBP/Blueprints/BP_MotionController Object Reference"))
  ;[1 1 1] Fire
  (set `self.IsFiring` true)
  (`self.Fire` :!label _label)
  (set `self.StillToWait` (`self.ShootTime`)))

(event `self.TriggerReleased`
  ;[1 1 1] Fire
  (set `self.IsFiring` false))

(event `self.ReceiveTick`
  (params (DeltaSeconds :type "Float (single-precision)"))
  ;[1 1 1] Fire
  (`parent.ReceiveTick` DeltaSeconds)
  (bind _output_get (set `self.StillToWait` (- (`self.StillToWait`) DeltaSeconds)))
  (if (and (<= _output_get 0.0) (`self.IsFiring`))
    (goto _label)))

(fn `UserConstructionScript`
  (`parent.UserConstructionScript`))