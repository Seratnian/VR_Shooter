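; BP_Weapon is a grabbable VR gun that fires physics bullets from a detachable magazine.
; It spawns and attaches a magazine at start, and when empty-slotted accepts an overlapping unused magazine of the matching class.
; Trigger pulls check remaining rounds, call the magazine's Fire, then spawn a bullet pushed by force.
; Grab release ejects the magazine through a shots-fired check; haptic feedback and inventory snippets are unwired.
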(event `self.MagazineArea.OnComponentBeginOverlap`
  (params (OverlappedComponent :type "PrimitiveComponent Object Reference") (OtherActor :type "Actor Object Reference") (OtherComp :type "PrimitiveComponent Object Reference") (OtherBodyIndex :type Integer) (bFromSweep :type Boolean) (SweepResult :type "HitResult Structure (by ref)"))
  ;[1 1 1] Pick up Magazine
  (bind _asbp_magazine (cast `/Game/Weapons/BP_Magazine` OtherActor))
  (`self.Pickup Magazine` _asbp_magazine))

(event `self.Pickup Magazine`
  (params (Magazine :type "/Game/Weapons/BP_Magazine Object Reference"))
  ;[1 1 1] Pick up Magazine
  ;;[1 1 1] check if magazine already exists
  (bind _hasmagazine (`self.GetHasMagazine`))
  (if (not _hasmagazine)
    ;;[1 1 1] Check if Magazine is fitting
    (if (== (`GameplayStatics.GetObjectClass` Magazine) (`self.MagazineClass`))
      ;;[1 1 1] check if new magazine is unused
      (if (`/Game/Sebastian/Blueprints/BP_Item.isNotUsed` Magazine)
        ;;[1 1 1] use magazine
        (`self.SetMagazine` Magazine)))))

(event `self.GrabReleased`
  (params (Controller :type "/Game/Sebastian/VirtualRealityBP/Blueprints/BP_MotionController Object Reference"))
  ;[1 1 1] Drop Magazine
  (`parent.GrabReleased` Controller)
  (`self.DropMagazine`))

(event `self.SetMagazine`
  (params (Magazine :type "/Game/Weapons/BP_Magazine Object Reference"))
  ;[1 1 1] Set Magazine
  (bind _output_get (set `self.Magazine` Magazine))
  (`/Engine/EditorBlueprintResources/StandardMacros.IsValid` _output_get
    (:`Is Valid`
      (set `/Game/Sebastian/Blueprints/BP_Item.isNotUsed` false _output_get)
      (`PrimitiveComponent.SetSimulatePhysics` (`/Game/Sebastian/Blueprints/BP_Item.Body` Magazine) false)
      (`SceneComponent.K2_AttachToComponent` (`Actor.RootComponent` Magazine) (`self.MagazineArea`) "None" "SnapToTarget" "SnapToTarget" "KeepWorld" true)
      (set `self.HasMagazine` true)
      (set `PrimitiveComponent.bGenerateOverlapEvents` false (`/Game/Sebastian/Blueprints/BP_Item.FirstHandArea` (`self.Magazine`))))))

(event `self.ReceiveBeginPlay`
  ;[1 1 1] Spawn Magazine
  (`parent.ReceiveBeginPlay`)
  (bind _magazine (`self.NewMagazine`))
  (`self.SetMagazine` _magazine))

(event `self.TriggerPulled`
  (params (Controller :type "/Game/Sebastian/VirtualRealityBP/Blueprints/BP_MotionController Object Reference"))
  ;[1 1 1] Fire
  (`self.Fire`))

(event `self.Fire`
  ;[1 1 1] Fire
  (bind _can_fire (`self.Can Fire`))
  (if _can_fire
    (`/Game/Weapons/BP_Magazine.Fire` (`self.Magazine`))
    (bind _returnvalue (`|SpawnActorFromClass` "/Game/Weapons/Bullets/BP_Bullet.BP_Bullet_C" (`KismetMathLibrary.MakeTransform` (.location (`SceneComponent.K2_GetComponentToWorld` (`self.Bullet Spawn Point`))) (.rotation (`SceneComponent.K2_GetComponentToWorld` (`self.Bullet Spawn Point`)))) "AlwaysSpawn" "OverrideRootScale" null null))
    (`PrimitiveComponent.AddForce` (`StaticMeshActor.StaticMeshComponent` _returnvalue) (* (`KismetMathLibrary.Conv_RotatorToVector` (`SceneComponent.K2_GetComponentRotation` (`self.Root`))) 500000.0) "None" false)
    (`KismetSystemLibrary.PrintString` "Fire")))

(event `/Game/Sebastian/VirtualRealityBP/Blueprints/PickupActorInterface.Drop`
  ;[1 1 1] Drop
  (`parent.Drop`)
  (set `self.isNotUsed` true)
  (set `PrimitiveComponent.bGenerateOverlapEvents` false (`self.FirstHandArea`)))

(fn `Can Fire`
  (returns (`Can Fire` :type Boolean))
  (bind _hasmagazine (`self.GetHasMagazine`))
  (if _hasmagazine
    (if (> (`/Game/Weapons/BP_Magazine.CurrentSize` (`self.Magazine`)) 0)
      (return true)
      (else
        _)))
  (return false))

(fn `DropMagazine`
  (returns (Dropped :type Boolean))
  (bind _magazine (`self.Magazine`))
  (`KismetSystemLibrary.PrintString` "drop mag")
  (bind _hasmagazine (`self.GetHasMagazine`))
  (if _hasmagazine
    (`/Game/Sebastian/Blueprints/Macros.TestMagazineIsFull` _magazine
      (:`Shots Fired`
        (set `/Game/Sebastian/Blueprints/BP_Item.isNotUsed` false _magazine)
        (`PrimitiveComponent.SetSimulatePhysics` (`/Game/Sebastian/Blueprints/BP_Item.Body` _magazine) true)
        (`SceneComponent.K2_DetachFromComponent` (`Actor.RootComponent` _magazine) "KeepWorld" "KeepWorld" "KeepWorld" true)
        (set `self.Magazine` null)
        (set `self.HasMagazine` false)
        (return true)))
    (else
      (return false))))

(fn `GetHasMagazine`
  (returns (HasMagazine :type Boolean))
  (return (`self.HasMagazine`)))

(fn `GetMagazine`
  (returns (Magazine :type "/Game/Weapons/BP_Magazine Object Reference"))
  (if (`self.HasMagazine`)
    (return (`self.Magazine`))
    (else
      (return null))))

(fn `NewMagazine`
  (returns (Magazine :type "/Game/Weapons/BP_Magazine Object Reference"))
  (bind _returnvalue (`|SpawnActorFromClass` (`self.MagazineClass`) (`KismetMathLibrary.MakeTransform` (0.0 0.0 0.0)) "AlwaysSpawn" "OverrideRootScale" null null))
  (return _returnvalue))

(fn `UserConstructionScript`)