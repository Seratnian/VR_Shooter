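; BP_Shotgun is a shotgun weapon Blueprint that fires a rapid burst of randomly spread shots each time it fires.
; Fire starts a burst only when BulletsFired is zero, so a new one cannot begin while the counter is running.
; PerformShot passes a random pitch and yaw within SprayArc to the parent's shot logic, then re-calls itself after a short Delay until BulletsPerShot is reached and the counter resets.
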(event `/Game/Weapons/Interface_Shooting.Fire`
  (if (== (`self.BulletsFired`) 0)
    (`self.Perform Shot` (struct))))

(event `self.Perform Shot`
  (params (Deviation :type "Rotator Structure"))
  (bind _spray_arc (`self.Spray Arc`))
  (bind _returnvalue (* _spray_arc -1.0))
  (`parent.Perform Shot` (`KismetMathLibrary.MakeRotator` 0.0 (`KismetMathLibrary.RandomFloatInRange` _returnvalue _spray_arc) (`KismetMathLibrary.RandomFloatInRange` _returnvalue _spray_arc)))
  (bind _result (`/Engine/EditorBlueprintResources/StandardMacros.IncrementInt` (`self.BulletsFired`))
    (:`  `
      (if (< _result (`self.Bullets Per Shot`))
        (`KismetSystemLibrary.Delay` 0.01)
        (`self.Perform Shot` (struct))
        (else
          (set `self.BulletsFired` 0))))))

(fn `UserConstructionScript`
  (`parent.UserConstructionScript`))