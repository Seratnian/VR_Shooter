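; BP_Rifle is a two-handed VR rifle that extends a parent weapon with second-hand grabbing and aiming.
; When a motion controller overlaps SecondHandArea while only the first hand holds the rifle, that controller grabs it as the second hand.
; Each tick with both hands holding, the root's pitch and yaw follow the line between the grab spheres, keeping its roll.
; CanFire defers to the parent only in a two-handed hold.
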(event `self.ReceiveTick`
  (params (DeltaSeconds :type "Float (single-precision)"))
  (bind _root (`self.Root`))
  ;[1 1 1] apply rotation
  (`parent.ReceiveTick` DeltaSeconds)
  (`/Game/Blueprints/Macros.Test First Hand` self
    (:`Is Held`
      (`/Game/Blueprints/Macros.Test Second Hand` self
        (:`Is Held`
          (`SceneComponent.K2_SetWorldRotation` _root (`KismetMathLibrary.MakeRotator` (.roll (`SceneComponent.K2_GetComponentRotation` _root)) (.pitch (`KismetMathLibrary.FindLookAtRotation` (`/Game/Blueprints/Macros.GetGrabSphereLocation` (`self.FirstHandController`)) (`/Game/Blueprints/Macros.GetGrabSphereLocation` (`self.SecondHandController`)))) (.yaw (`KismetMathLibrary.FindLookAtRotation` (`/Game/Blueprints/Macros.GetGrabSphereLocation` (`self.FirstHandController`)) (`/Game/Blueprints/Macros.GetGrabSphereLocation` (`self.SecondHandController`))))) false false))))))

(event `self.SecondHandArea.OnComponentBeginOverlap`
  (params (OverlappedComponent :type "PrimitiveComponent Object Reference") (OtherActor :type "Actor Object Reference") (OtherComp :type "PrimitiveComponent Object Reference") (OtherBodyIndex :type Integer) (bFromSweep :type Boolean) (SweepResult :type "HitResult Structure (by ref)"))
  ;[1 1 1] Let the secand hand grab the rifle
  (`/Game/Blueprints/Macros.Test First Hand` self
    (:`Is Held`
      (`/Game/Blueprints/Macros.Test Second Hand` self
        (:`Is Free`
          (bind _asbp_motion_controller (cast `/Game/VirtualRealityBP/Blueprints/BP_MotionController` OtherActor))
          (bind (_success _attachcomponent _attachactor) (`/Game/VirtualRealityBP/Blueprints/BP_MotionController.Grab SpecificActor` _asbp_motion_controller self))
          (if _success
            (set `self.SecondHandController` _attachactor)
            (set `self.IsInSecondHand` true)))))))

(fn `Can Fire`
  (returns (`Can Fire` :type Boolean))
  (`/Game/Blueprints/Macros.Test First Hand` self
    (:`Is Held`
      (`/Game/Blueprints/Macros.Test Second Hand` self
        (:`Is Held`
          (bind _can_fire (`parent.Can Fire`))
          (return _can_fire))
        (:`Is Free`
          _)))
    (:`Is Free`
      _))
  (return false))

(fn `UserConstructionScript`
  (`parent.UserConstructionScript`))