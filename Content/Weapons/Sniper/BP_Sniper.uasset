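; Sniper weapon Blueprint that adds a cycling scope zoom on top of its parent weapon's trigger behavior.
; A trigger pull from the second-hand controller advances the zoom mode through Near, Middle and Far, wrapping around, and sets the scene capture camera's field of view to match.
; Pulls from any other controller go to the parent's trigger handler, and CanFire always returns true.
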(event `/Game/Weapons/Interface_Shooting.TriggerPulled`
  (params (Controller :type "/Game/Sebastian/VirtualRealityBP/Blueprints/BP_MotionController Object Reference"))
  (`/Game/Sebastian/Blueprints/Macros.Test Object Equality` Controller (`self.SecondHandController`)
    (:`The Same`
      (bind _output_get (set `self.CurrentZoomState` (cast `/Game/Weapons/Sniper/ZoomMode` (mod (+ (`self.CurrentZoomState`) 1) (`KismetMathLibrary.Conv_IntToByte` (enumcount `/Game/Weapons/Sniper/ZoomMode`))))))
      (set `SceneCaptureComponent2D.FOVAngle` (select `/Game/Weapons/Sniper/ZoomMode` _output_get :`NewEnumerator0` 45.0 :`NewEnumerator1` 25.0 :`NewEnumerator2` 10.0 :!type "Float (single-precision)") (`self.SceneCaptureComponent2D`)))
    (:`Different`
      (`parent.TriggerPulled` Controller))))

(fn `Can Fire`
  (returns (`Can Fire` :type Boolean))
  (return true))

(fn `UserConstructionScript`
  (`parent.UserConstructionScript`))