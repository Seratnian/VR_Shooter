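; Grenade actor that a VR motion controller can grab; this graph holds no throw or explosion logic.
; On overlap with a BP_MotionController in a specific grip state, it has the controller grab it and tells the player pawn to remove it as an item.
; Pickup, called by the controller, disables mesh physics, then attaches and snaps the mesh to the given component.
; BeginPlay sets a DropTime that nothing here reads.
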(event `self.ReceiveBeginPlay`
  (set `self.DropTime` (`KismetMathLibrary.MakeTimespan` 0 0 0 0 1)))

(event `/Game/VirtualRealityBP/Blueprints/PickupActorInterface.Pickup`
  (params (AttachTo :type "SceneComponent Object Reference"))
  (`KismetSystemLibrary.PrintString` "Pickup")
  (`PrimitiveComponent.SetSimulatePhysics` (`self.StaticMeshComponent`) false)
  (`SceneComponent.K2_AttachToComponent` (`self.StaticMeshComponent`) AttachTo "None" "KeepWorld" "KeepWorld" "KeepWorld" false)
  (`SceneComponent.K2_SetWorldLocationAndRotation` (`self.StaticMeshComponent`) (`SceneComponent.K2_GetComponentLocation` AttachTo) (`SceneComponent.K2_GetComponentRotation` AttachTo) false false))

(event `self.ActorBeginOverlap`
  (params (OtherActor :type "Actor Object Reference"))
  (bind _asbp_motion_controller (cast `/Game/VirtualRealityBP/Blueprints/BP_MotionController` OtherActor))
  (if (`|EnumEquality` (`/Game/VirtualRealityBP/Blueprints/BP_MotionController.GripState` _asbp_motion_controller) "NewEnumerator2")
    (`/Game/VirtualRealityBP/Blueprints/BP_MotionController.Grab SpecificActor` _asbp_motion_controller self)
    (message `/Game/BP_Interface_Inventory.RemoveItemByObject` (`GameplayStatics.GetPlayerPawn` 0) self)))

(fn `UserConstructionScript`
  (`parent.UserConstructionScript`))