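; Post-processing Blueprint that drives gaze-based depth-of-field autofocus for the MotionControllerPawn's camera.
; BeginPlay caches the pawn and its camera; each Tick line-traces forward from the camera, with debug drawing, falling back to maximum range on a miss.
; Focal distance doubles or halves per frame toward that distance without overshooting, easing focus changes.
; Focal region is set equal to the new focal distance, while transition regions carry over.
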(event `self.ReceiveBeginPlay`
  (bind _asmotion_controller_pawn (cast `/Game/Sebastian/VirtualRealityBP/Blueprints/MotionControllerPawn` (`GameplayStatics.GetPlayerPawn` 0)))
  (set `self.MotionControllerPawn` _asmotion_controller_pawn)
  (set `self.Camera` (`/Game/Sebastian/VirtualRealityBP/Blueprints/MotionControllerPawn.Camera` _asmotion_controller_pawn)))

(event `self.ReceiveTick`
  (params (DeltaSeconds :type "Float (single-precision)"))
  (bind _camera (`self.Camera`))
  (bind _returnvalue (`SceneComponent.K2_GetComponentLocation` _camera))
  (bind _settings (`PostProcessComponent.Settings` (`self.Post Processing`)))
  (bind ((`DepthOfFieldFocalDistance` _depthoffieldfocaldistance)) (break `PostProcessSettings` _settings))
  (bind ((`DepthOfFieldMethod` _depthoffieldmethod) (`DepthOfFieldNearTransitionRegion` _depthoffieldneartransitionregion) (`DepthOfFieldFarTransitionRegion` _depthoffieldfartransitionregion)) (break `PostProcessSettings` _settings))
  (bind (_outhit _returnvalue_2) (`KismetSystemLibrary.LineTraceSingle` :`Start` _returnvalue :`End` (+ _returnvalue (`KismetMathLibrary.GreaterGreater_VectorRotator` (`KismetMathLibrary.MakeVector` 10000.0) (`SceneComponent.K2_GetComponentRotation` _camera))) :`TraceChannel` "TraceTypeQuery2" :`DrawDebugType` "ForOneFrame" :`DrawTime` 100.0))
  (bind _returnvalue_3 (select `bool` _returnvalue_2 :`false` 10000.0 :`true` (`.Distance` (`GameplayStatics.BreakHitResult` _outhit))))
  (bind _returnvalue_4 (> _returnvalue_3 _depthoffieldfocaldistance))
  (bind _returnvalue_5 (select `bool` _returnvalue_4 :`false` (/ _depthoffieldfocaldistance 2.0) :`true` (* _depthoffieldfocaldistance 2.0)))
  (bind _returnvalue_6 (select `bool` _returnvalue_4 :`false` (`KismetMathLibrary.FMax` _returnvalue_5 _returnvalue_3) :`true` (`KismetMathLibrary.FMin` _returnvalue_5 _returnvalue_3)))
  (set `PostProcessComponent.Settings` (make `PostProcessSettings` :`DepthOfFieldMethod` _depthoffieldmethod :`DepthOfFieldFocalDistance` _returnvalue_6 :`DepthOfFieldFocalRegion` (/ _returnvalue_6 1.0) :`DepthOfFieldNearTransitionRegion` _depthoffieldneartransitionregion :`DepthOfFieldFarTransitionRegion` _depthoffieldfartransitionregion) (`self.Post Processing`)))

(fn `UserConstructionScript`)