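; BP_Item is an item that motion controllers pick up, hold and drop.
; Overlapping FirstHandArea asks BP_MotionController to grab the item if it is pickable, then disables physics and snaps it to the returned attach component.
; While the item is in use, Tick drops it once grab has been held for DropTime, detaching it and restoring physics.
; SetIsInHand passes the held state recursively to attached BP_Items.
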(event `self.ReceiveTick`
  (params (DeltaSeconds :type "Float (single-precision)"))
  (`|ExecutionSequence`
    (:`then_1`
      ;[1 1 1] Check if should drop
      (`/Game/Sebastian/Blueprints/Macros.TestIfInHand` self
        (:`Is Used`
          (if (and (`self.IsGrabPressed`) (<= (+ (`self.DropStarted`) (`self.DropTime`)) (`KismetMathLibrary.Now`)))
            (`self.Drop`)))))))

(event `self.Drop`
  ;[1 1 1] Drop Item
  (`PrimitiveComponent.SetSimulatePhysics` (`self.Body`) true)
  (`self.K2_DetachFromActor` "KeepWorld" "KeepWorld" "KeepWorld")
  (set `/Game/Sebastian/VirtualRealityBP/Blueprints/BP_MotionController.AttachedActor` null (`self.FirstHandController`))
  (set `self.FirstHandController` null)
  (set `self.IsGrabPressed` false)
  (`self.SetIsInHand` false)
  (set `self.isNotUsed` false)
  (set `PrimitiveComponent.bGenerateOverlapEvents` false (`self.FirstHandArea`)))

(event `self.Pickup`
  (params (AttachTo :type "SceneComponent Object Reference") (Contoller :type "/Game/Sebastian/VirtualRealityBP/Blueprints/BP_MotionController Object Reference"))
  ;[1 1 1] Pick up Item
  (`self.SetIsInHand` true)
  (`PrimitiveComponent.SetSimulatePhysics` (`self.Body`) false)
  (`SceneComponent.K2_AttachToComponent` (`self.Root`) AttachTo "None" "SnapToTarget" "SnapToTarget" "KeepWorld" false))

(event `self.FirstHandArea.OnComponentBeginOverlap`
  (params (OverlappedComponent :type "PrimitiveComponent Object Reference") (OtherActor :type "Actor Object Reference") (OtherComp :type "PrimitiveComponent Object Reference") (OtherBodyIndex :type Integer) (bFromSweep :type Boolean) (SweepResult :type "HitResult Structure (by ref)"))
  ;[1 1 1] on collision with first hand area
  (bind (_is_possible _attach_component _attach_actor) (`self.IsPickupPossible` OtherActor))
  (if _is_possible
    (`self.Pickup` _attach_component _attach_actor)
    (set `self.FirstHandController` _attach_actor)))

(fn `Get Corresponding Inventory Item Class`
  (params (Items :type "Map of /Game/Sebastian/Blueprints/EnumInventoryPosition Enum to /Game/Sebastian/Blueprints/BP_Item Class Reference" :default _))
  (returns (` ` :type "Map of /Game/Sebastian/Blueprints/EnumInventoryPosition Enum to /Game/Sebastian/Blueprints/BP_Item Class Reference"))
  (return Items))

(fn `GrabPressed`
  (params (Controller :type "/Game/Sebastian/VirtualRealityBP/Blueprints/BP_MotionController Object Reference"))
  (set `self.IsGrabPressed` true)
  (set `self.DropStarted` (`KismetMathLibrary.Now`)))

(fn `GrabReleased`
  (params (Controller :type "/Game/Sebastian/VirtualRealityBP/Blueprints/BP_MotionController Object Reference"))
  (set `self.IsGrabPressed` false))

(fn `IsPickupPossible`
  (params (Controller :type "Actor Object Reference"))
  (returns (`Is Possible` :type Boolean) (`Attach Component` :type "MotionControllerComponent Object Reference") (`Attach Actor` :type "/Game/Sebastian/VirtualRealityBP/Blueprints/BP_MotionController Object Reference"))
  ;[1 1 1] Collide with controller
  (`/Game/Sebastian/Blueprints/Macros.TestIfPickable` self
    (:`Is Pickable`
      ;;[1 1 1] let the controller grab if desired and possible
      (bind _asbp_motion_controller (cast `/Game/Sebastian/VirtualRealityBP/Blueprints/BP_MotionController` Controller))
      (bind (_success _attachcomponent _attachactor) (`/Game/Sebastian/VirtualRealityBP/Blueprints/BP_MotionController.Grab SpecificActor` _asbp_motion_controller self))
      (return _success _attachcomponent _attachactor))
    (:`Not Pickable`
      (return false null null))))

(fn `SetIsInHand`
  (params (`IsInHand ` :type Boolean))
  (returns (` ` :type Boolean))
  (set `self.IsInFirstHand` `IsInHand `)
  (for _array_element (`self.GetAttachedActors`)
    (bind _asbp_item (cast `/Game/Sebastian/Blueprints/BP_Item` _array_element))
    (bind __ (`self.SetIsInHand` _asbp_item (`self.IsInFirstHand`)))
    (return __)))

(fn `UserConstructionScript`)